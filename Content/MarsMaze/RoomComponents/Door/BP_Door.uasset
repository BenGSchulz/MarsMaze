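; Sliding room door for MarsMaze that opens and closes together with a paired door.
; ActivateDoor toggles the state with audio and calls PairedActivate on the partner, or only plays a fail sound when no valid pair exists.
; PairedActivate toggles without audio or calling back, avoiding recursion.
; A timeline slides the mesh along its forward vector from the position cached at BeginPlay, reversing to close; opening also triggers air bursts.
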(event `self.ReceiveBeginPlay`
  (bind _doormesh (`self.DoorMesh`))
  (bind _output_get (set `self.ClosedLoc` (`SceneComponent.RelativeLocation` _doormesh)))
  (set `self.OpenedLoc` (+ _output_get (* (`KismetMathLibrary.GetForwardVector` (`SceneComponent.RelativeRotation` _doormesh)) 275.0))))

(event `OpenDoor`
  (bind (_direction _open_close) (`Timeline|OpenCloseTimeline` :!label _label)
    (:`Update`
      (`SceneComponent.K2_SetRelativeLocation` (`self.DoorMesh`) (`KismetMathLibrary.VLerp` (`self.ClosedLoc`) (`self.OpenedLoc`) _open_close) false false))))

(event `CloseDoor`
  (goto _label :!via `Reverse`))

(fn `ActivateDoor`
  (bind _audioclose (`self.AudioClose`))
  (bind _audioopen (`self.AudioOpen`))
  (if (`KismetSystemLibrary.IsValid` (`self.PairedDoor`))
    (`AudioComponent.Play` (`self.AudioInteractSuccess`) 0.0)
    (if (`self.Opened`)
      ;[1 1 1] Close
      (set `self.Opened` false)
      (if (`AudioComponent.IsPlaying` _audioopen)
        (`AudioComponent.Stop` _audioopen))
      (`AudioComponent.Play` (`self.AudioClose`) 0.0)
      (`self.CloseDoor`)
      (`self.PairedActivate` (`self.PairedDoor`))
      (else
        ;[1 1 1] Open
        (set `self.Opened` true)
        (if (`AudioComponent.IsPlaying` _audioclose)
          (`AudioComponent.Stop` _audioclose))
        (`AudioComponent.Play` (`self.AudioOpen`) 0.0)
        (`self.OpenDoor`)
        (`ActorComponent.Activate` (`self.AirBurst1`) false)
        (`ActorComponent.Activate` (`self.Airburst2`) false)
        (`self.PairedActivate` (`self.PairedDoor`))))
    (else
      (`AudioComponent.Play` (`self.AudioInteractFail`) 0.0))))

(fn `PairedActivate`
  (if (`self.Opened`)
    (set `self.Opened` false)
    (`self.CloseDoor`)
    (else
      (set `self.Opened` true)
      (`self.OpenDoor`)
      (`ActorComponent.Activate` (`self.AirBurst1`) false)
      (`ActorComponent.Activate` (`self.Airburst2`) false))))

(fn `UserConstructionScript`)