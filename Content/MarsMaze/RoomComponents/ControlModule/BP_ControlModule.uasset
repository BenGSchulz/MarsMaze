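; BP_ControlModule is the Mars Maze control module actor whose shutdown destroys it and wins the game.
; Shutdown plays click and beep sounds, then activates the spark and arc effects along with the Voltage audio.
; When that audio finishes, it hides the module and effects, flags itself destroyed and activates the explosion.
; After a short delay it calls WinGameEvent on the cached BP_MMGameMode.
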(event `self.ReceiveBeginPlay`
  (bind _asbp_mmgame_mode (cast `/Game/MarsMaze/Core/BP_MMGameMode` (`GameplayStatics.GetGameMode`)))
  (set `self.ThisGameMode` _asbp_mmgame_mode))

(event `self.Voltage.OnAudioFinished`
  (`SceneComponent.SetVisibility` (`self.Spark`) false false)
  (`SceneComponent.SetVisibility` (`self.Arc1`) false false)
  (`SceneComponent.SetVisibility` (`self.Arc2`) false false)
  (`SceneComponent.SetVisibility` (`self.Arc3`) false false)
  (`SceneComponent.SetVisibility` (`self.arc4`) false false)
  (`SceneComponent.SetVisibility` (`self.Module`) false false)
  (set `self.Destroyed` true)
  (`ActorComponent.Activate` (`self.Explosion`) false)
  (`ActorComponent.Activate` (`self.ExplosionPS`) false)
  (`KismetSystemLibrary.Delay` 1.0)
  (`/Game/MarsMaze/Core/BP_MMGameMode.WinGameEvent` (`self.ThisGameMode`)))

(fn `Shutdown`
  (`GameplayStatics.PlaySound2D` "/Game/MarsMaze/Audio/A_Click_Cue.A_Click_Cue" 1.0 1.0 0.0 null null)
  (`GameplayStatics.PlaySound2D` "/Game/MarsMaze/Audio/A_Beep_Cue.A_Beep_Cue" 1.0 1.0 0.0 null null)
  (`ActorComponent.Activate` (`self.Arc1`) false)
  (`ActorComponent.Activate` (`self.Arc2`) false)
  (`ActorComponent.Activate` (`self.Arc3`) false)
  (`ActorComponent.Activate` (`self.arc4`) false)
  (`ActorComponent.Activate` (`self.Spark`) false)
  (`ActorComponent.Activate` (`self.Voltage`) false))

(fn `UserConstructionScript`)