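; Mars Maze game mode that builds a random room maze at BeginPlay and handles game time, win and lose.
; Random wings branch from the center of a flattened grid, mixing plain and turret rooms, and the first dead end found becomes the control room.
; Grid cells spawn as room actors, null rooms filling gaps, then get neighbors and paired doors.
; Winning blends to an overhead camera before the menu; losing destroys the player.
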(event `self.ReceiveBeginPlay`
  ;[1 1 1] BeginPlay
  (bind _asbp_mmgame_instance (cast `/Game/MarsMaze/Core/BP_MMGameInstance` (`GameplayStatics.GetGameInstance`)))
  (set `self.ThisGameInstance` _asbp_mmgame_instance)
  ;;[1 1 1] Generate Map
  (`self.GenerateMap` 5)
  (`KismetSystemLibrary.PrintString` (`self.MapString`) false)
  (`self.SpawnRooms`)
  (`self.AssignNeighbors`)
  (`KismetSystemLibrary.K2_SetTimer` null "GameTimer" 1.0 true)
  (bind _returnvalue (`|SpawnActorFromClass` "/Script/Engine.CameraActor" (`KismetMathLibrary.MakeTransform` (0.0 5000.0 16000.0) (struct :`Pitch` -75.0 :`Yaw` -90.0)) "Undefined" "OverrideRootScale" null null))
  (set `self.OverviewCam` _returnvalue))

(event `self.ReceiveTick`
  (params (DeltaSeconds :type "Float (single-precision)")))

(event `WinGameEvent`
  (bind _returnvalue (`GameplayStatics.GetPlayerController` 0))
  (bind _thisgameinstance (`self.ThisGameInstance`))
  (`Widget.RemoveFromParent` (`/Game/MarsMaze/Core/BP_MMGameInstance.CharacterHUD` _thisgameinstance))
  (`GameplayStatics.PlaySound2D` "/Game/MarsMaze/Audio/A_Win_Cue.A_Win_Cue" 1.0 1.0 0.0 null null)
  (`PlayerController.SetViewTargetWithBlend` _returnvalue (`self.OverviewCam`) 3.0 "VTBlend_Linear" 0.0 false)
  (`KismetSystemLibrary.Delay` 3.0)
  (`UserWidget.AddToViewport` (`/Game/MarsMaze/Core/BP_MMGameInstance.WinMenu` _thisgameinstance) 0)
  (set `PlayerController.bShowMouseCursor` true _returnvalue))

(fn `AddWingMap`
  (params (StartRow :type Integer) (StartCol :type Integer))
  (returns (LastIndex :type "Array of Integer"))
  (locals (WingLength :type Integer) (Vertical :type Boolean) (Up :type Boolean) (Right :type Boolean))
  (bind _startrow (`local.StartRow`))
  (bind _startcol (`local.StartCol`))
  (bind _startrow_2 (`local.StartRow`))
  (bind _startrow_3 (`local.StartRow`))
  (bind _startcol_2 (`local.StartCol`))
  (bind _startcol_3 (`local.StartCol`))
  (bind _startcol_4 (`local.StartCol`))
  (bind _startcol_5 (`local.StartCol`))
  (bind _startrow_4 (`local.StartRow`))
  (bind _startrow_5 (`local.StartRow`))
  (bind _returnvalue (+ _startrow_2 (`local.WingLength`)))
  (bind _returnvalue_2 (+ _startcol (`local.WingLength`)))
  (bind _output_get (set `local.Vertical` (`KismetMathLibrary.RandomBool`)))
  (if _output_get
    ;[1 1 1] VerticalWing
    (set `local.WingLength` (`KismetMathLibrary.RandomInteger` (`KismetMathLibrary.Min` (- (+ (`self.MapSize`) 1) _startrow_3) _startrow_3)))
    (bind _output_get_2 (set `local.Up` (`KismetMathLibrary.RandomBool`)))
    (if _output_get_2
      (for _index (range _startrow_2 (+ _returnvalue 1))
        (bind _item (`self.IndexMap` _index _startcol_4))
        (if (== _item 0)
          (`self.InsertMap` _index (`local.StartCol`) (`KismetMathLibrary.RandomIntegerInRange` 2 3))))
      (return (`|MakeArray` _returnvalue _startcol_4))
      (else
        (for _index_2 (range (- _startrow (`local.WingLength`)) (+ _startrow 1))
          (bind _item_2 (`self.IndexMap` _index_2 _startcol_5))
          (if (== _item_2 0)
            (`self.InsertMap` _index_2 (`local.StartCol`) (`KismetMathLibrary.RandomIntegerInRange` 2 3))))
        (return (`|MakeArray` _startrow _startcol_5))))
    (else
      ;[1 1 1] HorizontalWing
      (set `local.WingLength` (`KismetMathLibrary.RandomInteger` (`KismetMathLibrary.Min` (- (`self.MapSize`) _startcol_2) _startcol_2)))
      (bind _output_get_3 (set `local.Right` (`KismetMathLibrary.RandomBool`)))
      (if _output_get_3
        (for _index_3 (range (- _startcol_3 (`local.WingLength`)) (+ _startcol_3 1))
          (bind _item_3 (`self.IndexMap` _startrow_4 _index_3))
          (if (== _item_3 0)
            (`self.InsertMap` (`local.StartRow`) _index_3 (`KismetMathLibrary.RandomIntegerInRange` 2 3))))
        (return (`|MakeArray` _startrow_4 _startcol_3))
        (else
          (for _index_4 (range _startcol (+ _returnvalue_2 1))
            (bind _item_4 (`self.IndexMap` _startrow_5 _index_4))
            (if (== _item_4 0)
              (`self.InsertMap` (`local.StartRow`) _index_4 (`KismetMathLibrary.RandomIntegerInRange` 2 3))))
          (return (`|MakeArray` _startrow_5 _returnvalue_2)))))))

(fn `AssignNeighbors`
  (locals (IndexOffsets :type "Array of Integer") (CurrRow :type Integer) (CurrCol :type Integer))
  (for _index (range (+ (`self.MapSize`) 1))
    (bind _output_get (set `local.CurrRow` _index))
    (for _index_2 (range (+ (`self.MapSize`) 1))
      (bind _output_get_2 (set `local.CurrCol` _index_2))
      (bind _room (`self.IndexRoom` _output_get _output_get_2))
      (if (not (== (`GameplayStatics.GetObjectClass` _room) "/Game/MarsMaze/Core/Rooms/BP_RoomBase_NullRoom.BP_RoomBase_NullRoom_C"))
        ;[1 1 1] For each index surrounding current room
        (for (_array_element _array_index) (`local.IndexOffsets`)
          (if (== (mod _array_index 2) 0)
            (bind _returnvalue (+ _array_element (`local.CurrRow`)))
            ;[1 1 1] Top and Bottom neighbors
            ;;[1 1 1] Check that neighbor index is in bounds
            (if (and (<= _returnvalue (`self.MapSize`)) (>= _returnvalue 0))
              (bind _room_2 (`self.IndexRoom` _returnvalue (`local.CurrCol`)))
              (bind _neighbors (`/Game/MarsMaze/Core/Rooms/BaseRoom/BP_RoomBase.Neighbors` _room))
              (`KismetArrayLibrary.Array_Add` _neighbors _room_2))
            (else
              (bind _returnvalue_2 (+ _array_element (`local.CurrCol`)))
              ;[1 1 1] Left and Right neighbors
              ;;[1 1 1] Check that neighbor index is in bounds
              (if (and (<= _returnvalue_2 (`self.MapSize`)) (>= _returnvalue_2 0))
                (bind _room_3 (`self.IndexRoom` (`local.CurrRow`) _returnvalue_2))
                (`KismetArrayLibrary.Array_Add` _neighbors _room_3))))))))
  (for _array_element_2 (`self.Rooms`)
    (if (not (== (`GameplayStatics.GetObjectClass` _array_element_2) "/Game/MarsMaze/Core/Rooms/BP_RoomBase_NullRoom.BP_RoomBase_NullRoom_C"))
      (`/Game/MarsMaze/Core/Rooms/BaseRoom/BP_RoomBase.PairDoors` _array_element_2))))

(fn `BranchMap`
  (params (RowIn :type Integer) (ColIn :type Integer) (BranchFactor :type Integer))
  (locals (IndexOffsets :type "Array of Integer") (RowToBranch :type Integer) (ColToBranch :type Integer) (RowsToBranch :type "Array of Integer") (ColsToBranch :type "Array of Integer") (BranchNum :type Integer))
  (bind _rowstobranch (`local.RowsToBranch`))
  (bind _colstobranch (`local.ColsToBranch`))
  (bind _branchnum (`local.BranchNum`))
  (bind _branchnum_2 (`local.BranchNum`))
  ;[1 1 1] Branching Spawn Point
  (set `local.BranchNum` BranchFactor)
  (`KismetArrayLibrary.Array_Add` (`local.RowsToBranch`) RowIn)
  (`KismetArrayLibrary.Array_Add` (`local.ColsToBranch`) ColIn)
  ;[1 1 1] While the arrays that hold branch locations are not empty,
  ; remove the first element of them and attempt to branch from that location
  (while (and (> (`KismetArrayLibrary.Array_Length` (`local.RowsToBranch`)) 0) (> (`KismetArrayLibrary.Array_Length` (`local.ColsToBranch`)) 0))
    (set `local.RowToBranch` (`|GetArrayItem` _rowstobranch))
    (`KismetArrayLibrary.Array_Remove` _rowstobranch)
    (set `local.ColToBranch` (`|GetArrayItem` _colstobranch))
    (`KismetArrayLibrary.Array_Remove` _colstobranch)
    ;[1 1 1] For each index surrounding player
    (for (_array_element _array_index) (`local.IndexOffsets`)
      (if (== (mod _array_index 2) 0)
        (bind _returnvalue (+ _array_element (`local.RowToBranch`)))
        ;[1 1 1] Top and Bottom neighbors
        ;;[1 1 1] Check that neighbor index is in bounds
        (if (and (< _returnvalue (`self.MapSize`)) (> _returnvalue 0))
          ;;[1 1 1] Add Wing at neighbor pos, if still branching, add last index on added wing to the indices to be branched later
          (bind _lastindex (`self.AddWingMap` _returnvalue (`local.ColToBranch`)))
          (if (> _branchnum_2 1)
            (`/Engine/EditorBlueprintResources/StandardMacros.DecrementInt` _branchnum_2
              (:`  `
                (`KismetArrayLibrary.Array_Add` (`local.RowsToBranch`) (`|GetArrayItem` _lastindex))
                (`KismetArrayLibrary.Array_Add` (`local.ColsToBranch`) (`|GetArrayItem` _lastindex 1))))))
        (else
          (bind _returnvalue_2 (+ _array_element (`local.ColToBranch`)))
          ;[1 1 1] Left and Right neighbors
          ;;[1 1 1] Check that neighbor index is in bounds
          (if (and (< _returnvalue_2 (`self.MapSize`)) (> _returnvalue_2 0))
            ;;[1 1 1] Add Wing at neighbor pos. If still branching, add last index on added wing to the indices to be branched later
            (bind _lastindex_2 (`self.AddWingMap` (`local.RowToBranch`) _returnvalue_2))
            (if (> _branchnum 1)
              (`/Engine/EditorBlueprintResources/StandardMacros.DecrementInt` _branchnum
                (:`  `
                  (`KismetArrayLibrary.Array_Add` (`local.RowsToBranch`) (`|GetArrayItem` _lastindex_2))
                  (`KismetArrayLibrary.Array_Add` (`local.ColsToBranch`) (`|GetArrayItem` _lastindex_2 1)))))))))))

(fn `GameTimer`
  (if (not (`/Game/MarsMaze/Core/BP_MMGameInstance.InMenu` (`self.ThisGameInstance`)))
    (bind _result (`/Engine/EditorBlueprintResources/StandardMacros.IncrementInt` (`self.GameTime`))
      (:`  `
        (`KismetSystemLibrary.PrintString` (`KismetStringLibrary.Conv_IntToString` _result) false)))))

(fn `GenerateMap`
  (params (BranchFactor :type Integer))
  (locals (RandomVal :type Integer) (CenterIndex :type Integer))
  (bind _centerindex (`local.CenterIndex`))
  (bind _returnvalue (* (+ (`self.MapSize`) 1) (+ (`self.MapSize`) 1)))
  (set `local.CenterIndex` (/ (`self.MapSize`) 2))
  (`KismetArrayLibrary.Array_Resize` (`self.RoomMap`) _returnvalue)
  (`KismetArrayLibrary.Array_Resize` (`self.Rooms`) _returnvalue)
  (for _index (range (+ (`self.MapSize`) 1))
    (for _index_2 (range (+ (`self.MapSize`) 1))
      (`self.InsertMap` _index_2 _index)))
  (`self.InsertMap` _centerindex _centerindex 1)
  (`self.BranchMap` _centerindex _centerindex (`local.BranchFactor`))
  (`self.InsertControlMap`)
  (`self.MapToString`))

(fn `IndexMap`
  (params (Row :type Integer) (Col :type Integer))
  (returns (Item :type Integer))
  (return (`|GetArrayItem` (`self.RoomMap`) (+ (* (+ (`self.MapSize`) 1) Row) Col))))

(fn `IndexRoom`
  (params (Row :type Integer) (Col :type Integer))
  (returns (Room :type "/Game/MarsMaze/Core/Rooms/BaseRoom/BP_RoomBase Object Reference"))
  (return (`|GetArrayItem` (`self.Rooms`) (+ (* (+ (`self.MapSize`) 1) Row) Col))))

(fn `InsertControlMap`
  (locals (IndexOffsets :type "Array of Integer") (CurrRow :type Integer) (CurrCol :type Integer) (NeighborCount :type Integer))
  (for _index (range (+ (`self.MapSize`) 1))
    (bind _output_get (set `local.CurrRow` _index))
    (for _index_2 (range (+ (`self.MapSize`) 1))
      (bind _output_get_2 (set `local.CurrCol` _index_2))
      (bind _item (`self.IndexMap` _output_get _output_get_2))
      (if (!= _item 0)
        ;[1 1 1] For each index surrounding current room
        (for (_array_element _array_index) (`local.IndexOffsets`)
          (if (== (mod _array_index 2) 0)
            (bind _returnvalue (+ _array_element (`local.CurrRow`)))
            ;[1 1 1] Top and Bottom neighbors
            ;;[1 1 1] Check that neighbor index is in bounds
            (if (and (<= _returnvalue (`self.MapSize`)) (>= _returnvalue 0))
              (bind _item_2 (`self.IndexMap` _returnvalue (`local.CurrCol`)))
              (if (!= _item_2 0)
                (`/Engine/EditorBlueprintResources/StandardMacros.IncrementInt` (`local.NeighborCount`))))
            (else
              (bind _returnvalue_2 (+ _array_element (`local.CurrCol`)))
              ;[1 1 1] Left and Right neighbors
              ;;[1 1 1] Check that neighbor index is in bounds
              (if (and (<= _returnvalue_2 (`self.MapSize`)) (>= _returnvalue_2 0))
                (bind _item_3 (`self.IndexMap` (`local.CurrRow`) _returnvalue_2))
                (if (!= _item_3 0)
                  (`/Engine/EditorBlueprintResources/StandardMacros.IncrementInt` (`local.NeighborCount`)))))))
        (if (== (`local.NeighborCount`) 1)
          (`self.InsertMap` (`local.CurrRow`) (`local.CurrCol`) 4)
          (return)
          (else
            (set `local.NeighborCount` 0)))))))

(fn `InsertMap`
  (params (Row :type Integer) (Col :type Integer) (Val :type Integer))
  (`KismetArrayLibrary.Array_Set` (`self.RoomMap`) (+ (* (+ (`self.MapSize`) 1) Row) Col) Val))

(fn `InsertRoom`
  (params (Row :type Integer) (Col :type Integer) (In :type "/Game/MarsMaze/Core/Rooms/BaseRoom/BP_RoomBase Object Reference"))
  (`KismetArrayLibrary.Array_Set` (`self.Rooms`) (+ (* (+ (`self.MapSize`) 1) Row) Col) In))

(fn `LoseGame`
  (bind _thisgameinstance (`self.ThisGameInstance`))
  (`Widget.RemoveFromParent` (`/Game/MarsMaze/Core/BP_MMGameInstance.CharacterHUD` _thisgameinstance))
  (`self.K2_DestroyActor` (`GameplayStatics.GetPlayerCharacter` 0))
  (`GameplayStatics.PlaySound2D` "/Game/MarsMaze/Audio/A_Lose_Cue.A_Lose_Cue" 1.0 1.0 0.0 null null)
  (`UserWidget.AddToViewport` (`/Game/MarsMaze/Core/BP_MMGameInstance.LoseMenu` _thisgameinstance) 0)
  (set `PlayerController.bShowMouseCursor` true (`GameplayStatics.GetPlayerController` 0)))

(fn `MapToString`
  (set `self.MapString` " \n")
  (for _index (range (+ (`self.MapSize`) 1))
    (for _index_2 (range (+ (`self.MapSize`) 1))
      (bind _item (`self.IndexMap` _index _index_2))
      (set `self.MapString` (`KismetStringLibrary.Concat_StrStr` (`self.MapString`) (`KismetStringLibrary.Conv_IntToString` _item) ", ")))
    (set `self.MapString` (`KismetStringLibrary.Concat_StrStr` (`self.MapString`) " \n"))))

(fn `RoomsToString`
  (set `self.RoomString` " \n")
  (for _index (range (+ (`self.MapSize`) 1))
    (for _index_2 (range (+ (`self.MapSize`) 1))
      (bind _room (`self.IndexRoom` _index _index_2))
      (set `self.RoomString` (`KismetStringLibrary.Concat_StrStr` (`self.RoomString`) (`KismetSystemLibrary.GetObjectName` _room) ", ")))
    (set `self.RoomString` (`KismetStringLibrary.Concat_StrStr` (`self.RoomString`) " \n"))))

(fn `SpawnRooms`
  (locals (CurrRow :type Integer) (CurrCol :type Integer))
  (bind _returnvalue (`KismetMathLibrary.MakeTransform` (`KismetMathLibrary.MakeVector` (* (- (`local.CurrCol`) (`self.Center`)) 1260.0) (* (- (- (`local.CurrRow`) 1) (`self.Center`)) 1260.0) 100.0)))
  ;[1 1 1] Spawn Rooms
  (for _index (range (+ (`self.MapSize`) 1))
    (set `local.CurrRow` _index)
    (for _index_2 (range (+ (`self.MapSize`) 1))
      (set `local.CurrCol` _index_2)
      (bind _item (`self.IndexMap` (`local.CurrRow`) (`local.CurrCol`)))
      (switch `int` _item
        (:`0`
          (bind _returnvalue_2 (`|SpawnActorFromClass` "/Game/MarsMaze/Core/Rooms/BP_RoomBase_NullRoom.BP_RoomBase_NullRoom_C" (`KismetMathLibrary.MakeTransform` (0.0 0.0 -1000.0)) "Undefined" "OverrideRootScale" null null))
          (`self.InsertRoom` (`local.CurrRow`) (`local.CurrCol`) _returnvalue_2))
        (:`1`
          (bind _returnvalue_3 (`|SpawnActorFromClass` "/Game/MarsMaze/Core/Rooms/BaseRoom/BP_RoomBase.BP_RoomBase_C" _returnvalue "Undefined" "OverrideRootScale" null null :!label _label))
          (`self.InsertRoom` (`local.CurrRow`) (`local.CurrCol`) _returnvalue_3))
        (:`2`
          (goto _label))
        (:`3`
          (bind _returnvalue_4 (`|SpawnActorFromClass` "/Game/MarsMaze/Core/Rooms/TurretRoom/BP_TurretRoom.BP_TurretRoom_C" _returnvalue "Undefined" "OverrideRootScale" null null))
          (`self.InsertRoom` (`local.CurrRow`) (`local.CurrCol`) _returnvalue_4))
        (:`4`
          (bind _returnvalue_5 (`|SpawnActorFromClass` "/Game/MarsMaze/Core/Rooms/ControlRoom/BP_RoomBase_ControlRoom.BP_RoomBase_ControlRoom_C" _returnvalue "Undefined" "OverrideRootScale" null null))
          (`self.InsertRoom` (`local.CurrRow`) (`local.CurrCol`) _returnvalue_5))))))

(fn `UserConstructionScript`)

(fn `WinGame`
  (`Widget.RemoveFromParent` (`/Game/MarsMaze/Core/BP_MMGameInstance.CharacterHUD` (`self.ThisGameInstance`)))
  (`PlayerController.SetViewTargetWithBlend` (`GameplayStatics.GetPlayerController` 0) null 0.0 "VTBlend_Linear" 0.0 false))