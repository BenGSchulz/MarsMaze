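; Game instance for MarsMaze that creates and holds the game's shared UI widgets.
; On Init, a sequence creates the main menu, character HUD, lose, win, pause and status alert widgets and stores each in a variable.
; It then sets a Loaded flag once all of them are created.
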(event `self.ReceiveInit`
  (`|ExecutionSequence`
    (:`then_0`
      (bind _returnvalue (`|CreateWidget` "/Game/MarsMaze/UI/MainMenuUI.MainMenuUI_C"))
      (set `self.MainMenu` _returnvalue))
    (:`then_1`
      (bind _returnvalue_2 (`|CreateWidget` "/Game/MarsMaze/Core/Character/WBP_CharacterHUD.WBP_CharacterHUD_C"))
      (set `self.CharacterHUD` _returnvalue_2))
    (:`then_2`
      (bind _returnvalue_3 (`|CreateWidget` "/Game/MarsMaze/UI/LoseMenuUI.LoseMenuUI_C"))
      (set `self.LoseMenu` _returnvalue_3))
    (:`then_3`
      (bind _returnvalue_4 (`|CreateWidget` "/Game/MarsMaze/UI/WinMenuUI.WinMenuUI_C"))
      (set `self.WinMenu` _returnvalue_4))
    (:`then_4`
      (bind _returnvalue_5 (`|CreateWidget` "/Game/MarsMaze/UI/PauseMenuUI.PauseMenuUI_C"))
      (set `self.PauseMenu` _returnvalue_5))
    (:`then_5`
      (bind _returnvalue_6 (`|CreateWidget` "/Game/MarsMaze/UI/StatusAlertUI.StatusAlertUI_C"))
      (set `self.StatusAlert` _returnvalue_6))
    (:`then_6`
      (set `self.Loaded` true))))