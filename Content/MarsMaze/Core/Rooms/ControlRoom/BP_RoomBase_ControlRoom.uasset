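; BP_RoomBase_ControlRoom is the control room variant of the room base in MarsMaze, housing a control module and an alarm.
; On BeginPlay it spawns a BP_ControlModule at a fixed offset and attaches it to itself.
; Tick polls the module's Destroyed flag and the game instance's InMenu flag, restarting the alarm outside menus while the module survives and stopping it once the module is destroyed.
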(event `self.ReceiveBeginPlay`
  (`parent.ReceiveBeginPlay`)
  (bind _returnvalue (`|SpawnActorFromClass` "/Game/MarsMaze/RoomComponents/ControlModule/BP_ControlModule.BP_ControlModule_C" (`KismetMathLibrary.MakeTransform` (0.0 1260.0 0.0)) "Undefined" "OverrideRootScale" null null))
  (bind _output_get (set `self.ControlModule` _returnvalue))
  (`self.K2_AttachToActor` _output_get self "None" "KeepRelative" "KeepRelative" "KeepRelative" true))

(event `self.ReceiveTick`
  (params (DeltaSeconds :type "Float (single-precision)"))
  (bind _alarm (`self.Alarm`))
  (bind _returnvalue (`AudioComponent.IsPlaying` _alarm))
  (bind _destroyed (`/Game/MarsMaze/RoomComponents/ControlModule/BP_ControlModule.Destroyed` (`self.ControlModule`)))
  (`parent.ReceiveTick` DeltaSeconds)
  (bind _asbp_mmgame_instance (cast `/Game/MarsMaze/Core/BP_MMGameInstance` (`GameplayStatics.GetGameInstance`)))
  (if (not (`/Game/MarsMaze/Core/BP_MMGameInstance.InMenu` _asbp_mmgame_instance))
    (if (and (not _returnvalue) (not _destroyed))
      (`AudioComponent.Play` _alarm 0.0)
      (else
        (if _destroyed :!label _label
          (if _returnvalue
            (`AudioComponent.Stop` _alarm)))))
    (else
      (goto _label))))

(fn `UserConstructionScript`
  (`parent.UserConstructionScript`))