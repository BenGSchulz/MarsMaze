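; BP_RoomBase is a maze room actor that owns its doors and tracks whether the player is inside.
; On BeginPlay it spawns and attaches a room trigger and one door per DoorTransforms entry.
; Tick polls the trigger's overlap with the player pawn to set PlayerInRoom.
; PairDoors links each door to the opposite door of its neighbor via a four-way index offset, skipping BP_RoomBase_NullRoom neighbors.
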(event `self.ReceiveBeginPlay`
  ;[1 1 1] BeginPlay
  ;;[1 1 1] Spawn and attach room trigger
  (bind _returnvalue (`|SpawnActorFromClass` "/Game/MarsMaze/RoomComponents/BP_RoomTriggerBase.BP_RoomTriggerBase_C" (`KismetMathLibrary.MakeTransform` (0.0 1260.0 250.0)) "Undefined" "OverrideRootScale" null null))
  (`self.K2_AttachToActor` _returnvalue self "None" "KeepRelative" "KeepRelative" "KeepWorld" true)
  (set `self.RoomTrigger` _returnvalue)
  ;;[1 1 1] Spawn and attach doors
  (for _array_element (`self.DoorTransforms`)
    (bind _returnvalue_2 (`|SpawnActorFromClass` "/Game/MarsMaze/RoomComponents/Door/BP_Door.BP_Door_C" _array_element "Undefined" "OverrideRootScale" null null))
    (`self.K2_AttachToActor` _returnvalue_2 self "None" "KeepRelative" "KeepWorld" "KeepWorld" true)
    (`KismetArrayLibrary.Array_Add` (`self.Doors`) _returnvalue_2)))

(event `self.ReceiveTick`
  (params (DeltaSeconds :type "Float (single-precision)"))
  ;[1 1 1] TICK
  ;;[1 1 1] Check if player in room using spawned room trigger
  (set `self.PlayerInRoom` (`self.IsOverlappingActor` (`self.RoomTrigger`) (`Controller.K2_GetPawn` (`GameplayStatics.GetPlayerController` 0)))))

(fn `PairDoors`
  (for (_array_element _array_index) (`self.Neighbors`)
    (if (not (== (`GameplayStatics.GetObjectClass` _array_element) "/Game/MarsMaze/Core/Rooms/BP_RoomBase_NullRoom.BP_RoomBase_NullRoom_C"))
      (set `/Game/MarsMaze/RoomComponents/Door/BP_Door.PairedDoor` (`|GetArrayItem` (`/Game/MarsMaze/Core/Rooms/BaseRoom/BP_RoomBase.Doors` _array_element) (mod (+ _array_index 2) 4)) (`|GetArrayItem` (`self.Doors`) _array_index)))))

(fn `UserConstructionScript`)