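; BP_Character is the player character for MarsMaze, with walking, jogging, jumping, crouch toggling and camera look.
; Each tick a short sphere trace from the view camera, ignoring overlapped room triggers, identifies door switches or control modules by component name.
; The Interact input then activates the focused door or shuts down the module.
; TakeDamage lowers health; at zero, Tick plays a death sound and, after a delay, tells the game mode the game is lost.
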(event `self.ReceiveBeginPlay`
  ;[1 1 1] BeginPlay
  (bind _asbp_mmgame_mode (cast `/Game/MarsMaze/Core/BP_MMGameMode` (`GameplayStatics.GetGameMode`)))
  (set `self.ThisGameMode` _asbp_mmgame_mode)
  (set `self.CurrentHealth` (`self.MaxHealth`)))

(event `self.ReceiveTick`
  (params (DeltaSeconds :type "Float (single-precision)"))
  (bind _viewcamera (`self.ViewCamera`))
  (bind _returnvalue (`SceneComponent.K2_GetComponentLocation` _viewcamera))
  ;[1 1 1] TICK
  (`|ExecutionSequence`
    (:`then_0`
      ;;[1 1 1] Send Spherecast for button interaction
      (bind (_outhit _returnvalue_2) (`KismetSystemLibrary.SphereTraceSingleForObjects` _returnvalue (+ _returnvalue (* (`KismetMathLibrary.GetForwardVector` (`SceneComponent.K2_GetComponentRotation` _viewcamera)) 300.0)) 5.0 (`|MakeArray` "ObjectTypeQuery2" :!type "EObjectTypeQuery Enum") false (`PrimitiveComponent.GetOverlappingActors` (`self.CapsuleComponent`) "/Game/MarsMaze/RoomComponents/BP_RoomTriggerBase.BP_RoomTriggerBase_C")))
      (if _returnvalue_2
        (bind (_bblockinghit _binitialoverlap _time _distance _location _impactpoint _normal _impactnormal _physmat _hitactor _hitcomponent) (`GameplayStatics.BreakHitResult` _outhit))
        (switch `string` (`KismetSystemLibrary.GetObjectName` _hitcomponent)
          (:`Default`
            (set `self.InteractionObject` "NewEnumerator2" :!label _label))
          (:`DoorSwitch`
            (set `self.InteractionObject` "NewEnumerator0")
            (set `self.FocusedActor` _hitactor :!label _label_2))
          (:`Module`
            (set `self.InteractionObject` "NewEnumerator1")
            (goto _label_2)))
        (else
          (goto _label))))
    (:`then_1`
      (if (and (<= (`self.CurrentHealth`) 0.0) (not (`self.Dead`)))
        (set `self.Dead` true)
        (`GameplayStatics.PlaySound2D` "/Game/MarsMaze/Audio/A_Death_Cue.A_Death_Cue" 1.0 1.0 0.0 null null)
        (`KismetSystemLibrary.Delay` 3.0)
        (`/Game/MarsMaze/Core/BP_MMGameMode.LoseGame` (`self.ThisGameMode`))))))

(event `InputAxis|MoveForward`
  (params (AxisValue :type "Float (single-precision)"))
  ;[1 1 1] Character Movement
  ;;[1 1 1] WASD Movement
  (if (not (`self.DisableMovement`))
    (`self.AddMovementInput` (`KismetMathLibrary.GetForwardVector` (`KismetMathLibrary.MakeRotator` 0.0 0.0 (.yaw (`self.GetControlRotation`)))) AxisValue)))

(event `InputAction|Jog`
  (params (Key :type "Key Structure"))
  (bind _biscrouched (`self.bIsCrouched`))
  (bind _charactermovement (`self.CharacterMovement`))
  ;[1 1 1] Character Movement
  ;;[1 1 1] Jogging
  (:`Pressed`
    (set `self.JogPressed` true)
    (if _biscrouched
      (set `CharacterMovementComponent.MaxWalkSpeedCrouched` 300.0 _charactermovement)
      (else
        (set `CharacterMovementComponent.MaxWalkSpeed` 600.0 _charactermovement))))
  (:`Released`
    (set `self.JogPressed` false)
    (if _biscrouched
      (set `CharacterMovementComponent.MaxWalkSpeedCrouched` 200.0 _charactermovement)
      (else
        (set `CharacterMovementComponent.MaxWalkSpeed` 400.0 _charactermovement)))))

(event `InputAxis|MoveRight`
  (params (AxisValue :type "Float (single-precision)"))
  ;[1 1 1] Character Movement
  ;;[1 1 1] WASD Movement
  (if (not (`self.DisableMovement`))
    (`self.AddMovementInput` (`KismetMathLibrary.GetRightVector` (`KismetMathLibrary.MakeRotator` 0.0 0.0 (.yaw (`self.GetControlRotation`)))) AxisValue)))

(event `InputAction|Jump`
  (params (Key :type "Key Structure"))
  (bind _charactermovement (`self.CharacterMovement`))
  ;[1 1 1] Character Movement
  ;;[1 1 1] Jumping
  (:`Pressed`
    (set `self.JumpPressed` true)
    (if (`self.DisableMovement`)
      _
      (elif (not (`self.bIsCrouched`))
        (if (> (`KismetMathLibrary.VSize` (`MovementComponent.Velocity` (`self.CharacterMovement`))) 0.0)
          (set `CharacterMovementComponent.JumpZVelocity` 350.0 _charactermovement)
          (else
            (set `CharacterMovementComponent.JumpZVelocity` 325.0 _charactermovement)))
        (`self.Jump`))))
  (:`Released`
    (set `self.JumpPressed` false)))

(event `InputAxis|Turn`
  (params (AxisValue :type "Float (single-precision)"))
  ;[1 1 1] Character Movement
  ;;[1 1 1] Look Around
  (`self.AddControllerYawInput` AxisValue))

(event `InputAction|Crouch`
  (params (Key :type "Key Structure"))
  ;[1 1 1] Character Movement
  ;;[1 1 1] Crouching
  (:`Pressed`
    (`/Engine/EditorBlueprintResources/StandardMacros.FlipFlop`
      (:`A`
        (`self.Crouch`))
      (:`B`
        (`self.UnCrouch`)))))

(event `InputAxis|LookUp`
  (params (AxisValue :type "Float (single-precision)"))
  ;[1 1 1] Character Movement
  ;;[1 1 1] Look Around
  (`self.AddControllerPitchInput` AxisValue))

(event `InputAction|Interact`
  (params (Key :type "Key Structure"))
  (bind _focusedactor (`self.FocusedActor`))
  ;[1 1 1] Interaction
  (:`Pressed`
    (set `self.InteractPressed` true)
    (switch `/Game/MarsMaze/Core/Character/EInteractionObject` (`self.InteractionObject`)
      (:`NewEnumerator0`
        (bind _asbp_door (cast `/Game/MarsMaze/RoomComponents/Door/BP_Door` _focusedactor))
        (`/Game/MarsMaze/RoomComponents/Door/BP_Door.ActivateDoor` _asbp_door))
      (:`NewEnumerator1`
        (bind _asbp_control_module (cast `/Game/MarsMaze/RoomComponents/ControlModule/BP_ControlModule` _focusedactor))
        (`/Game/MarsMaze/RoomComponents/ControlModule/BP_ControlModule.Shutdown` _asbp_control_module))))
  (:`Released`
    (set `self.InteractPressed` false)))

(fn `TakeDamage`
  (params (Amount :type "Float (double-precision)"))
  (set `self.CurrentHealth` (- (`self.CurrentHealth`) Amount))
  (if (not (`self.TakenDamage`))
    (set `self.TakenDamage` true)))

(fn `UserConstructionScript`)