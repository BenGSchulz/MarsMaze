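; BP_LaserShot is a laser projectile from the Mars Maze turret AI that damages the player character on overlap.
; Its collider ignores itself and room triggers, then on a BP_Character applies fixed damage, plays a grunt and destroys the shot after a short delay.
; A looping timer counts TimeAlive in tenth-of-a-second steps, and Tick destroys the shot once it reaches LifeTime.
; The hit sound and destroy logic for other impacts is disconnected.
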(event `self.ReceiveBeginPlay`
  (`KismetSystemLibrary.K2_SetTimer` null "LifeTimer" 0.1 true))

(event `LifeTimer`
  (set `self.TimeAlive` (+ (`self.TimeAlive`) 1.0)))

(event `self.ReceiveTick`
  (params (DeltaSeconds :type "Float (single-precision)"))
  (if (not (< (`self.TimeAlive`) (`self.LifeTime`)))
    (`self.K2_DestroyActor`)))

(event `self.Collider.OnComponentBeginOverlap`
  (params (OverlappedComponent :type "PrimitiveComponent Object Reference") (OtherActor :type "Actor Object Reference") (OtherComp :type "PrimitiveComponent Object Reference") (OtherBodyIndex :type Integer) (bFromSweep :type Boolean) (SweepResult :type "HitResult Structure (by ref)"))
  (if (and (!= OtherActor self) (!= (`GameplayStatics.GetObjectClass` OtherActor) "/Game/MarsMaze/RoomComponents/BP_RoomTriggerBase.BP_RoomTriggerBase_C"))
    (bind _asbp_character (cast `/Game/MarsMaze/Core/Character/BP_Character` OtherActor))
    (`/Game/MarsMaze/Core/Character/BP_Character.TakeDamage` _asbp_character 10.0)
    (`GameplayStatics.PlaySound2D` "/Game/MarsMaze/Audio/A_Grunt_Cue.A_Grunt_Cue" 1.0 1.0 0.0 null null)
    (`KismetSystemLibrary.Delay` 0.1)
    (`self.K2_DestroyActor`)))

(fn `UserConstructionScript`)