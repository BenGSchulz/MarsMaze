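; Turret actor for the Mars maze game that fires laser shots through its Fire function.
; Fire plays the laser sound, activates the muzzle particle effect and spawns a BP_LaserShot with the turret as instigator.
; The LaserSound component doubles as the muzzle point, giving the spawn transform and the forward impulse on the shot's collider.
; The event graph holds no logic, so targeting and fire timing are not handled in these graphs.
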(event `self.ReceiveTick`
  (params (DeltaSeconds :type "Float (single-precision)")))

(fn `Fire`
  (bind _lasersound (`self.LaserSound`))
  (`AudioComponent.Play` (`self.LaserSound`) 0.0)
  (`ActorComponent.Activate` (`self.PS_LaserShoot`) false)
  (bind _returnvalue (`|SpawnActorFromClass` "/Game/MarsMaze/AI/Turret/Components/BP_LaserShot.BP_LaserShot_C" (`SceneComponent.K2_GetComponentToWorld` _lasersound) "AlwaysSpawn" "OverrideRootScale" null self))
  (`PrimitiveComponent.AddImpulse` (`/Game/MarsMaze/AI/Turret/Components/BP_LaserShot.Collider` _returnvalue) (* (`SceneComponent.GetForwardVector` _lasersound) 1500.0) "None" false))

(fn `UserConstructionScript`)